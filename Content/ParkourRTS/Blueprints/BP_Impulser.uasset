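; BP_Impulser is a short-lived explosion impulse that knocks the player character (Benny) away.
; BeginPlay plays an explosion sound, then destroys the actor after a brief delay.
; Tick animates the Impulser component by steadily subtracting from its world scale, labeled as visual expansion.
; When that component hits the player, it overwrites the character's movement velocity with a large vector along the negated impact normal.
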(event `self.ReceiveBeginPlay`
  (`GameplayStatics.PlaySound2D` "/Game/ParkourRTS/External_Imports/Sound/Explosion_Cue.Explosion_Cue" 1.0 1.0 0.0 null null)
  ;[1 1 1] Destroy after creation.
  (`KismetSystemLibrary.Delay` 0.4)
  (`self.K2_DestroyActor`))

(event `self.ReceiveTick`
  (params (DeltaSeconds :type "Float (single-precision)"))
  ;[1 1 1] Visual Expansion
  (`SceneComponent.SetWorldScale3D` (`self.Impulser`) (- (`SceneComponent.K2_GetComponentScale` (`self.Impulser`)) (* DeltaSeconds 15.0))))

(event `self.Impulser.OnComponentHit`
  (params (HitComponent :type "PrimitiveComponent Object Reference") (OtherActor :type "Actor Object Reference") (OtherComp :type "PrimitiveComponent Object Reference") (NormalImpulse :type "Vector Structure") (Hit :type "HitResult Structure (by ref)"))
  (bind _returnvalue (`GameplayStatics.GetPlayerCharacter` 0))
  ;[1 1 1] Push Benny Away from impulse
  (if (== OtherActor _returnvalue)
    (set `MovementComponent.Velocity` (* (`.ImpactNormal` (`GameplayStatics.BreakHitResult` Hit)) -8000.0) (`Character.CharacterMovement` _returnvalue))))

(fn `UserConstructionScript`)