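; BP_LightsOut is a self-destroying actor that briefly blacks out the level when spawned.
; On BeginPlay, a delay-timed sequence plays pop and snap cues, flicks a switch mesh via its morph target, and zeroes the intensity of the DirectionalLight found by class lookup.
; Seconds later it flips the switch back, restores a hard-coded intensity rather than the original, adds a tinnitus cue and destroys itself.
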(event `self.ReceiveBeginPlay`
  (`GameplayStatics.PlaySound2D` "/Game/ParkourRTS/Custom_Imports/Audio/pop_Cue.pop_Cue" 1.0 1.0 0.0 null null)
  (`KismetSystemLibrary.Delay` 0.4)
  (`GameplayStatics.PlaySound2D` "/Game/ParkourRTS/Custom_Imports/Audio/Snap_Cue.Snap_Cue" 1.0 1.0 0.0 null null)
  (`SkeletalMeshComponent.SetMorphTarget` (`self.Switch`) "FLICK" 1.0 true)
  (`KismetSystemLibrary.Delay` 0.4)
  (bind _returnvalue (`GameplayStatics.GetActorOfClass` "/Script/Engine.DirectionalLight"))
  (`LightComponent.SetIntensity` (`Light.LightComponent` _returnvalue) 0.0)
  (`KismetSystemLibrary.Delay` 6.0)
  (`SkeletalMeshComponent.SetMorphTarget` (`self.Switch`) "FLICK" 0.0 true)
  (`GameplayStatics.PlaySound2D` "/Game/ParkourRTS/Custom_Imports/Audio/Snap_Cue.Snap_Cue" 1.0 1.0 0.0 null null)
  (`GameplayStatics.PlaySound2D` "/Game/ParkourRTS/Custom_Imports/Audio/Tinnitus_Cue.Tinnitus_Cue" 0.5 1.0 0.0 null null)
  (bind _returnvalue_2 (`GameplayStatics.GetActorOfClass` "/Script/Engine.DirectionalLight"))
  (`LightComponent.SetIntensity` (`Light.LightComponent` _returnvalue_2) 10.0)
  (`KismetSystemLibrary.Delay` 0.4)
  (`self.K2_DestroyActor`))

(fn `UserConstructionScript`)