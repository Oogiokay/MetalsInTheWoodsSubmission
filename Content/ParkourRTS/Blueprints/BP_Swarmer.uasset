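; BP_Swarmer is a short-lived homing bee actor that chases the player character.
; Every tick it rotates the Bee component to face the player's capsule and applies a physics impulse in that direction, so movement is physics-driven.
; After a random delay of a few seconds from BeginPlay, it destroys itself and plays a 2D pop sound.
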(event `self.ReceiveBeginPlay`
  (`KismetSystemLibrary.Delay` (`KismetMathLibrary.RandomFloatInRange` 3.0 5.0))
  (`self.K2_DestroyActor`)
  (`GameplayStatics.PlaySound2D` "/Game/ParkourRTS/Custom_Imports/Audio/pop_Cue.pop_Cue" 1.0 1.0 0.0 null null))

(event `self.ReceiveTick`
  (params (DeltaSeconds :type "Float (single-precision)"))
  (bind _bee (`self.Bee`))
  (bind _returnvalue (`KismetMathLibrary.FindLookAtRotation` (`SceneComponent.K2_GetComponentLocation` _bee) (`SceneComponent.K2_GetComponentLocation` (`Character.CapsuleComponent` (`GameplayStatics.GetPlayerCharacter` 0)))))
  (`SceneComponent.K2_SetWorldRotation` _bee _returnvalue false false)
  (`PrimitiveComponent.AddImpulse` (`self.Bee`) (* (`KismetMathLibrary.GetForwardVector` _returnvalue) 3000.0) "None" false))

(fn `UserConstructionScript`)