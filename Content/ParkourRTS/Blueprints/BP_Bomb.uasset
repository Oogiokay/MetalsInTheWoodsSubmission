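; Bomb actor that spawns a BP_Impulser as its explosion, on a timer or on contact with the player.
; It sets the explosion class on BeginPlay, then calls SpawnThing and destroys itself after a short fuse delay.
; Hitting the player character triggers the same sequence immediately.
; Other impacts play a quiet 2D clinking sound when the normal impulse is strong enough.
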(event `self.ReceiveBeginPlay`
  (`parent.ReceiveBeginPlay`)
  (set `self.ExplosionClass` "/Game/ParkourRTS/Blueprints/BP_Impulser.BP_Impulser_C")
  (`KismetSystemLibrary.Delay` 5.0)
  (`self.SpawnThing`)
  (`self.K2_DestroyActor`))

(event `self.Object.OnComponentHit`
  (params (HitComponent :type "PrimitiveComponent Object Reference") (OtherActor :type "Actor Object Reference") (OtherComp :type "PrimitiveComponent Object Reference") (NormalImpulse :type "Vector Structure") (Hit :type "HitResult Structure (by ref)"))
  (if (== OtherActor (`GameplayStatics.GetPlayerCharacter` 0))
    (`self.SpawnThing`)
    (`self.K2_DestroyActor`)
    (else
      (`/Engine/EditorBlueprintResources/StandardMacros.CompareFloat` (`KismetMathLibrary.VSize` NormalImpulse) 2000.0
        (:`>`
          (`GameplayStatics.PlaySound2D` "/Game/ParkourRTS/External_Imports/Sound/Clinks/Clinking.Clinking" 0.05 1.0 0.0 null null))))))

(event `self.Object.OnComponentBeginOverlap`
  (params (OverlappedComponent :type "PrimitiveComponent Object Reference") (OtherActor :type "Actor Object Reference") (OtherComp :type "PrimitiveComponent Object Reference") (OtherBodyIndex :type Integer) (bFromSweep :type Boolean) (SweepResult :type "HitResult Structure (by ref)")))

(fn `UserConstructionScript`
  (`parent.UserConstructionScript`))