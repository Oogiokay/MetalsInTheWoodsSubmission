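; BP_AbilityBase is the base ability Blueprint for the Wizard Ability System, providing shared cooldown and charge handling.
; ActivateAbility spends a charge, sets the cooldown flag and starts a named timer that calls EndCooldown to clear it and print a debug message.
; Its return value is inverted: true means blocked by cooldown or empty charges, false means activated.
; Charges are never replenished here, and several debug prints sit disconnected.
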(fn `ActivateAbility`
  (returns (WontFire :type Boolean))
  ;[1 1 1] Handles Cooldown & Charges
  (if (`self.IsOnCooldown`)
    (return true)
    (elif (> (`self.Charges`) 0)
      (set `self.IsOnCooldown` true)
      (`/Engine/EditorBlueprintResources/StandardMacros.DecrementInt` (`self.Charges`)
        (:`  `
          (`KismetSystemLibrary.K2_SetTimer` null "EndCooldown" (`self.Cooldown`)) ; My beloved timer
          (return false)))
      (else
        (return true)))))

(fn `EndCooldown`
  (set `self.IsOnCooldown` false)
  (`KismetSystemLibrary.PrintString` (`KismetStringLibrary.Concat_StrStr` (`KismetSystemLibrary.GetObjectName` self) " Is off cooldown") true true (struct :`G` 0.66 :`B` 1.0 :`A` 1.0) 2.0 "sfafdasdasdasd"))

(fn `UserConstructionScript`)