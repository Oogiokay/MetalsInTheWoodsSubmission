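; Wizard ability Blueprint for Lights Out, part of the Parkour RTS wizard ability system.
; When the parent ActivateAbility returns false, it spawns a BP_LightsOut actor at a fixed raised world location and returns false.
; The wizard lookup on that path is unused.
; Older logic that zeroes and restores DirectionalLight intensity is disconnected, leaving ResetIntensity without a live caller here.
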(fn `ActivateAbility`
  (returns (WontFire :type Boolean))
  (bind _wontfire (`parent.ActivateAbility`))
  (if (not _wontfire)
    (`GameplayStatics.GetActorOfClass` "/Game/ParkourRTS/Blueprints/GamePlay/BP_RTSParkour_Wizard.BP_RTSParkour_Wizard_C") ; Get William
    (`|SpawnActorFromClass` "/Game/ParkourRTS/Blueprints/BP_LightsOut.BP_LightsOut_C" (`KismetMathLibrary.MakeTransform` (0.0 0.0 1400.0)) "AlwaysSpawn" "MultiplyWithRoot" null null) ; Spawn Swarmers From William
    (return false)))

(fn `ResetIntensity`
  (bind _returnvalue (`GameplayStatics.GetActorOfClass` "/Script/Engine.DirectionalLight"))
  (`LightComponent.SetIntensity` (`Light.LightComponent` _returnvalue) 10.0))

(fn `UserConstructionScript`
  (`parent.UserConstructionScript`))