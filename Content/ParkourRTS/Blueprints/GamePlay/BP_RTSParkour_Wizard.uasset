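; Wizard actor for the RTS parkour game that wraps around the play area in the XZ plane.
; Every tick, Bounds compares the root component's world X and Z against the BottomLeftBounds and TopRightBounds vectors.
; Crossing an edge teleports the root to the opposite edge on that axis, keeping the other coordinates, for screen-wrap style movement.
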(event `self.ReceiveTick`
  (params (DeltaSeconds :type "Float (single-precision)"))
  (`self.Bounds`))

(fn `Bounds`
  (bind (_bottomleftbounds_x _bottomleftbounds_y _bottomleftbounds_z) (`KismetMathLibrary.BreakVector` (`self.BottomLeftBounds`)))
  (bind (_toprightbounds_x _toprightbounds_y _toprightbounds_z) (`KismetMathLibrary.BreakVector` (`self.TopRightBounds`)))
  (bind _toprightbounds_x_2 (`KismetMathLibrary.BreakVector` (`self.TopRightBounds`)))
  (bind (_bottomleftbounds_x_2 _bottomleftbounds_y_2 _bottomleftbounds_z_2) (`KismetMathLibrary.BreakVector` (`self.BottomLeftBounds`)))
  (bind (_toprightbounds_x_3 _toprightbounds_y_2 _toprightbounds_z_2) (`KismetMathLibrary.BreakVector` (`self.TopRightBounds`)))
  (bind _bottomleftbounds_x_3 (`KismetMathLibrary.BreakVector` (`self.BottomLeftBounds`)))
  (bind (_returnvalue_x _returnvalue_y) (`KismetMathLibrary.BreakVector` (`SceneComponent.K2_GetComponentLocation` (`self.DefaultSceneRoot`))))
  (bind (_returnvalue_x_2 _returnvalue_y_2 _returnvalue_z) (`KismetMathLibrary.BreakVector` (`SceneComponent.K2_GetComponentLocation` (`self.DefaultSceneRoot`))))
  (bind (_returnvalue_x_3 _returnvalue_y_3) (`KismetMathLibrary.BreakVector` (`SceneComponent.K2_GetComponentLocation` (`self.DefaultSceneRoot`))))
  (bind (_returnvalue_x_4 _returnvalue_y_4 _returnvalue_z_2) (`KismetMathLibrary.BreakVector` (`SceneComponent.K2_GetComponentLocation` (`self.DefaultSceneRoot`))))
  (bind (_returnvalue_x_5 _returnvalue_y_5 _returnvalue_z_3) (`KismetMathLibrary.BreakVector` (`SceneComponent.K2_GetComponentLocation` (`self.DefaultSceneRoot`))))
  (set `self.WorldX` _returnvalue_x_5)
  (set `self.WorldZ` _returnvalue_z_3)
  (`|ExecutionSequence`
    (:`then_0`
      (if (< (`self.WorldX`) _bottomleftbounds_x)
        (`SceneComponent.K2_SetWorldLocation` (`self.DefaultSceneRoot`) (`KismetMathLibrary.MakeVector` _toprightbounds_x_2 _returnvalue_y_4 _returnvalue_z_2) false false)))
    (:`then_1`
      (if (> (`self.WorldX`) _toprightbounds_x)
        (`SceneComponent.K2_SetWorldLocation` (`self.DefaultSceneRoot`) (`KismetMathLibrary.MakeVector` _bottomleftbounds_x_3 _returnvalue_y_2 _returnvalue_z) false false)))
    (:`then_2`
      (if (< (`self.WorldZ`) _bottomleftbounds_z)
        (`SceneComponent.K2_SetWorldLocation` (`self.DefaultSceneRoot`) (`KismetMathLibrary.MakeVector` _returnvalue_x_3 _returnvalue_y_3 _toprightbounds_z_2) false false)))
    (:`then_3`
      (if (> (`self.WorldZ`) _toprightbounds_z)
        (`SceneComponent.K2_SetWorldLocation` (`self.DefaultSceneRoot`) (`KismetMathLibrary.MakeVector` _returnvalue_x _returnvalue_y _bottomleftbounds_z_2) false false)))))

(fn `UserConstructionScript`)