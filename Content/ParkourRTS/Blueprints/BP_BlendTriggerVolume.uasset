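; Trigger volume that blends the player's view between a static camera and the parkour character's third-person camera.
; BeginPlay switches the character's controller to the first BP_StaticCamera found in the level, regardless of overlap.
; Entering OverlapVolume blends to that static camera; leaving it blends back to the character.
; All switches use SetViewTargetWithBlend with a shared blend time, and overlaps only react to BP_RTSParkour_Character.
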(event `self.ReceiveBeginPlay`
  (bind _returnvalue (`GameplayStatics.GetActorOfClass` "/Game/ParkourRTS/Blueprints/GamePlay/BP_RTSParkour_Character.BP_RTSParkour_Character_C"))
  (bind _asbp_rtsparkour_character (cast `/Game/ParkourRTS/Blueprints/GamePlay/BP_RTSParkour_Character` _returnvalue))
  (if (`KismetSystemLibrary.IsValid` _asbp_rtsparkour_character)
    (bind _asplayer_controller (cast `PlayerController` (`Pawn.GetController` _asbp_rtsparkour_character)))
    (bind _returnvalue_2 (`GameplayStatics.GetActorOfClass` "/Game/ParkourRTS/Blueprints/GamePlay/BP_StaticCamera.BP_StaticCamera_C"))
    (`PlayerController.SetViewTargetWithBlend` _asplayer_controller _returnvalue_2 (`self.CameraBlendTme`) "VTBlend_Linear" 0.0 false)))

(event `self.OverlapVolume.OnComponentWake`
  (params (WakingComponent :type "PrimitiveComponent Object Reference") (BoneName :type Name)))

(event `self.OverlapVolume.OnComponentBeginOverlap`
  (params (OverlappedComponent :type "PrimitiveComponent Object Reference") (OtherActor :type "Actor Object Reference") (OtherComp :type "PrimitiveComponent Object Reference") (OtherBodyIndex :type Integer) (bFromSweep :type Boolean) (SweepResult :type "HitResult Structure (by ref)"))
  ;[1 1 1] Sets the Camera View to the found Example Camera BP
  (bind _asbp_rtsparkour_character (cast `/Game/ParkourRTS/Blueprints/GamePlay/BP_RTSParkour_Character` OtherActor))
  (if (`KismetSystemLibrary.IsValid` _asbp_rtsparkour_character)
    (bind _asplayer_controller (cast `PlayerController` (`Pawn.GetController` _asbp_rtsparkour_character)))
    (if (`KismetSystemLibrary.IsValid` _asplayer_controller)
      (bind _returnvalue (`GameplayStatics.GetActorOfClass` "/Game/ParkourRTS/Blueprints/GamePlay/BP_StaticCamera.BP_StaticCamera_C"))
      (`PlayerController.SetViewTargetWithBlend` _asplayer_controller _returnvalue (`self.CameraBlendTme`) "VTBlend_Linear" 0.0 false))))

(event `self.OverlapVolume.OnComponentEndOverlap`
  (params (OverlappedComponent :type "PrimitiveComponent Object Reference") (OtherActor :type "Actor Object Reference") (OtherComp :type "PrimitiveComponent Object Reference") (OtherBodyIndex :type Integer))
  ;[1 1 1] Resets the Camera View to the Third Person Camera
  (bind _asbp_rtsparkour_character (cast `/Game/ParkourRTS/Blueprints/GamePlay/BP_RTSParkour_Character` OtherActor))
  (if (`KismetSystemLibrary.IsValid` _asbp_rtsparkour_character)
    (bind _asplayer_controller (cast `PlayerController` (`Pawn.GetController` _asbp_rtsparkour_character)))
    (if (`KismetSystemLibrary.IsValid` _asplayer_controller)
      (`PlayerController.SetViewTargetWithBlend` _asplayer_controller _asbp_rtsparkour_character (`self.CameraBlendTme`) "VTBlend_Linear" 0.0 false))))

(fn `UserConstructionScript`)