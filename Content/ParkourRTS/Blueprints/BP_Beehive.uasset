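; BP_Beehive is a beehive actor that bursts into a swarm by spawning things in a loop sized by SwarmSize, then destroys itself.
; BeginPlay runs the parent logic, sets ExplosionClass to BP_Swarmer and triggers the burst after a short delay.
; A hit on its Object component runs the same spawn-and-destroy sequence without waiting for the delay.
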(event `self.ReceiveBeginPlay`
  (`parent.ReceiveBeginPlay`)
  (set `self.ExplosionClass` "/Game/ParkourRTS/Blueprints/BP_Swarmer.BP_Swarmer_C")
  (`KismetSystemLibrary.Delay` 2.0)
  (for _ (range (+ (`self.SwarmSize`) 1))
    (`self.SpawnThing`))
  (`self.K2_DestroyActor`))

(event `self.Object.OnComponentHit`
  (params (HitComponent :type "PrimitiveComponent Object Reference") (OtherActor :type "Actor Object Reference") (OtherComp :type "PrimitiveComponent Object Reference") (NormalImpulse :type "Vector Structure") (Hit :type "HitResult Structure (by ref)"))
  (for _ (range (+ (`self.SwarmSize`) 1))
    (`self.SpawnThing`))
  (`self.K2_DestroyActor`))

(fn `UserConstructionScript`
  (`parent.UserConstructionScript`))