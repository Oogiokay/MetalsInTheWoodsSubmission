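; Wizard Blueprint for ParkourRTS that keeps its Sphere component inside a rectangular area with screen-wrap style movement.
; Every Tick it runs Bounds, which compares the Sphere's world position with the BottomLeftBounds and TopRightBounds vectors on the X and Z axes.
; Crossing an edge teleports the Sphere to the opposite edge on that axis, leaving the other coordinates unchanged.
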(event `self.ReceiveTick`
  (params (DeltaSeconds :type "Float (single-precision)"))
  (`self.Bounds`))

(fn `Bounds`
  (bind (_bottomleftbounds_x _bottomleftbounds_y _bottomleftbounds_z) (`KismetMathLibrary.BreakVector` (`self.BottomLeftBounds`)))
  (bind (_toprightbounds_x _toprightbounds_y _toprightbounds_z) (`KismetMathLibrary.BreakVector` (`self.TopRightBounds`)))
  (bind _toprightbounds_x_2 (`KismetMathLibrary.BreakVector` (`self.TopRightBounds`)))
  (bind _sphere (`self.Sphere`))
  (bind _sphere_2 (`self.Sphere`))
  (bind (_bottomleftbounds_x_2 _bottomleftbounds_y_2 _bottomleftbounds_z_2) (`KismetMathLibrary.BreakVector` (`self.BottomLeftBounds`)))
  (bind (_toprightbounds_x_3 _toprightbounds_y_2 _toprightbounds_z_2) (`KismetMathLibrary.BreakVector` (`self.TopRightBounds`)))
  (bind _sphere_3 (`self.Sphere`))
  (bind _sphere_4 (`self.Sphere`))
  (bind _bottomleftbounds_x_3 (`KismetMathLibrary.BreakVector` (`self.BottomLeftBounds`)))
  (bind (_returnvalue_x _returnvalue_y) (`KismetMathLibrary.BreakVector` (`SceneComponent.K2_GetComponentLocation` _sphere_3)))
  (bind (_returnvalue_x_2 _returnvalue_y_2 _returnvalue_z) (`KismetMathLibrary.BreakVector` (`SceneComponent.K2_GetComponentLocation` _sphere_4)))
  (bind (_returnvalue_x_3 _returnvalue_y_3) (`KismetMathLibrary.BreakVector` (`SceneComponent.K2_GetComponentLocation` _sphere_2)))
  (bind (_returnvalue_x_4 _returnvalue_y_4 _returnvalue_z_2) (`KismetMathLibrary.BreakVector` (`SceneComponent.K2_GetComponentLocation` _sphere)))
  (bind (_returnvalue_x_5 _returnvalue_y_5 _returnvalue_z_3) (`KismetMathLibrary.BreakVector` (`SceneComponent.K2_GetComponentLocation` (`self.Sphere`))))
  (`|ExecutionSequence`
    (:`then_0`
      (if (< _returnvalue_x_5 _bottomleftbounds_x)
        (`SceneComponent.K2_SetWorldLocation` _sphere (`KismetMathLibrary.MakeVector` _toprightbounds_x_2 _returnvalue_y_4 _returnvalue_z_2) false false)))
    (:`then_1`
      (if (> _returnvalue_x_5 _toprightbounds_x)
        (`SceneComponent.K2_SetWorldLocation` _sphere_4 (`KismetMathLibrary.MakeVector` _bottomleftbounds_x_3 _returnvalue_y_2 _returnvalue_z) false false)))
    (:`then_2`
      (if (< _returnvalue_z_3 _bottomleftbounds_z)
        (`SceneComponent.K2_SetWorldLocation` _sphere_2 (`KismetMathLibrary.MakeVector` _returnvalue_x_3 _returnvalue_y_3 _toprightbounds_z_2) false false)))
    (:`then_3`
      (if (> _returnvalue_z_3 _toprightbounds_z)
        (`SceneComponent.K2_SetWorldLocation` _sphere_3 (`KismetMathLibrary.MakeVector` _returnvalue_x _returnvalue_y _bottomleftbounds_z_2) false false)))))

(fn `UserConstructionScript`)